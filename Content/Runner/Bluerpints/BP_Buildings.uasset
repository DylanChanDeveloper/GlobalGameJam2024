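; BP_Buildings is a runner-game segment that adds a building child actor during construction and exposes its Arrow transform as an attach point.
; SpawnBuildings switches between six spawn points, SP1 to SP6, but its selector is fixed so only SP6 is used, leaving a random-integer node unconnected.
; The box overlap event, noted for extending the floor, only casts to BP_RunnerGameMode and does nothing further.
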(event OnComponentBeginOverlap(BoxCollsion)
  (params (OverlappedComponent :type Primitive%20Component%20Object%20Reference) (OtherActor :type Actor%20Object%20Reference) (OtherComp :type Primitive%20Component%20Object%20Reference) (OtherBodyIndex :type Integer) (bFromSweep :type Boolean) (SweepResult :type Hit%20Result%20Structure%20%28by%20ref%29))
  ;[1 1 1] Exend Floor
  (Utilities|Casting|CastToBP_RunnerGameMode (Game|GetGameMode)))

(event EventBeginPlay)

(event Collision|EventActorBeginOverlap
  (params (OtherActor :type Actor%20Object%20Reference)))

(event EventTick
  (params (DeltaSeconds :type Float%20%28single-precision%29)))

(fn ConstructionScript
  (CallFunction|SpawnBuildings))

(fn GetAttachPoint
  (return (Transformation|GetWorldTransform (Variables|Default|GetArrow))))

(fn SpawnBuildings
  (Utilities|FlowControl|Sequence
    (:then_0
      (switch int 5
        (:0
          (AddComponent|AddChildActorComponent false (Transformation|GetRelativeTransform (Variables|Default|GetSP1))))
        (:1
          (AddComponent|AddChildActorComponent false (Transformation|GetRelativeTransform (Variables|Default|GetSP2))))
        (:2
          (AddComponent|AddChildActorComponent false (Transformation|GetRelativeTransform (Variables|Default|GetSP3))))
        (:3
          (AddComponent|AddChildActorComponent false (Transformation|GetRelativeTransform (Variables|Default|GetSP4))))
        (:4
          (AddComponent|AddChildActorComponent false (Transformation|GetRelativeTransform (Variables|Default|GetSP5))))
        (:5
          (AddComponent|AddChildActorComponent false (Transformation|GetRelativeTransform (Variables|Default|GetSP6))))))))