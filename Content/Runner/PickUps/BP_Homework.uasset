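; BP_Homework is a runner-game pickup that counts as a coin when the player character touches it.
; On overlap with BP_RunnerCharacter, it increments the game mode's Coins, prints the total, plays a scribble sound, destroys itself and calls the character's UpdateCoins.
; It also destroys itself without awarding anything when it overlaps a BP_Obsticles_Wall obstacle.
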(event EventBeginPlay)

(event Collision|EventActorBeginOverlap
  (params (OtherActor :type Actor%20Object%20Reference))
  (Utilities|FlowControl|Sequence
    (:then_0
      (bind _asbp_runner_character (Utilities|Casting|CastToBP_RunnerCharacter OtherActor))
      (bind _asbp_runner_game_mode (Utilities|Casting|CastToBP_RunnerGameMode (Game|GetGameMode)))
      (bind _result (Math|Integer|IncrementInt (Variables|/Game/Runner/Bluerpints/BP_RunnerGameMode.BP_RunnerGameMode_C|GetCoins _asbp_runner_game_mode))
        (:%20%20
          (Development|PrintString (Utilities|String|ToString(Integer) _result))
          (Audio|PlaySound2D "/Game/WaveSounds/scribble-6144.scribble-6144" 1.0 1.0 0.0 0 0)
          (Actor|DestroyActor)
          (Default|UpdateCoins _asbp_runner_character))))
    (:then_1
      (Utilities|Casting|CastToBP_Obsticles_Wall OtherActor)
      (Actor|DestroyActor))))

(event EventTick
  (params (DeltaSeconds :type Float%20%28single-precision%29)))

(fn ConstructionScript)